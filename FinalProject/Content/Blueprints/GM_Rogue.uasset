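; GM_Rogue is a game mode that tracks score and remaining enemies per level, with the enemy count equal to LevelIndex.
; Each BP_Bee kill adds its Value to Score, and clearing all enemies below level index 4 opens the LevelClear widget in UI-only input.
; OnLevelLoad resets the count and restores game-only input.
; SpawnEnemy places a bee above the player, and Tick prints the level index for debugging.
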(event EventBeginPlay
  (Variables|Default|SetEnemyCount (Variables|Default|GetLevelIndex)))

(event EventTick
  (params (DeltaSeconds :type Float%20%28single-precision%29))
  (Utilities|FlowControl|Delay 1.0)
  (Development|PrintString (Utilities|String|Append "Current index" (Utilities|String|ToString(Integer) (Variables|Default|GetLevelIndex)))))

(fn ConstructionScript)

(fn SpawnEnemy
  (Game|SpawnActorfromClass "/Game/Blueprints/Characters/BP_Bee.BP_Bee_C" (Math|Conversions|ToTransform(Vector) (+ (Transformation|GetWorldLocation (Variables|/Script/Engine.Actor|GetRootComponent (Game|GetPlayerCharacter 0))) "0.000000,0.100000,200.000000")) "Undefined" "MultiplyWithRoot" 0 0))

(fn OnEnemyKilled
  (params (Enemy :type Character%20Object%20Reference))
  (bind _asbp_bee (Utilities|Casting|CastToBP_Bee Enemy))
  (Variables|Default|SetScore (+ (Variables|Default|GetScore) (Variables|/Game/Blueprints/Characters/BP_Bee.BP_Bee_C|Getvalue _asbp_bee)))
  (bind _output_get (Variables|Default|SetEnemyCount (- (Variables|Default|GetEnemyCount) 1)))
  (if (== _output_get 0)
    (if (not (>= (Variables|Default|GetLevelIndex) 4))
      (CallFunction|OnLevelClear))))

(fn OnLevelClear
  (bind _returnvalue (Game|GetPlayerController 0))
  (Development|PrintString "level clear")
  (bind _returnvalue_2 (UserInterface|CreateWidget "/Game/Blueprints/UI/LevelClear.LevelClear_C"))
  (UserInterface|Viewport|AddtoViewport _returnvalue_2 0)
  (Variables|/Script/Engine.PlayerController|SetbShowMouseCursor _returnvalue true)
  (Input|SetInputModeUIOnly _returnvalue _returnvalue_2 "DoNotLock" false))

(fn OnLevelLoad
  (bind _returnvalue (Game|GetPlayerController 0))
  (Variables|Default|SetEnemyCount (Variables|Default|GetLevelIndex))
  (Variables|/Script/Engine.PlayerController|SetbShowMouseCursor _returnvalue true)
  (Input|SetInputModeGameOnly _returnvalue false))