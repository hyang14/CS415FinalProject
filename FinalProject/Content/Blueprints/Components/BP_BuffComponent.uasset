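; BP_BuffComponent is a component that stores active buffs and tracks their remaining time.
; AddBuff appends a new buff instance with the definition's duration and one stack, without merging duplicates, and GetBuffs returns the list.
; Tick subtracts delta time from each instance, skipping those at -1, and rebuilds its struct in the array.
; Expired buffs are not removed, and no buff effects are applied here.
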(event EventBeginPlay)

(event EventTick
  (params (DeltaSeconds :type Float%20%28single-precision%29))
  (bind _activatedbuffs (Variables|Default|GetActivatedBuffs))
  (for (_array_element _array_index) _activatedbuffs
    (if (not (== (.remaintime _array_element) -1.0))
      (Utilities|Array|SetArrayElem _activatedbuffs _array_index (Utilities|Struct|MakeST_BuffInstance (.buff_def (Utilities|Array|Get(acopy) _activatedbuffs _array_index)) (- (.remaintime (Utilities|Array|Get(acopy) _activatedbuffs _array_index)) DeltaSeconds) (.stackcnt (Utilities|Array|Get(acopy) _activatedbuffs _array_index)))))))

(fn AddBuff
  (params (BufDef :type ST%20Buff%20Definition%20Structure))
  (Utilities|Array|Add (Variables|Default|GetActivatedBuffs) (Utilities|Struct|MakeST_BuffInstance BufDef (.Duration (Utilities|Struct|BreakST_BuffDefinition BufDef)) 1)))

(fn GetBuffs
  (return (Variables|Default|GetActivatedBuffs)))