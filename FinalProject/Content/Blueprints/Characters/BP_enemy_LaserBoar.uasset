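; Laser Boar enemy that moves along X, roaming and chasing the player with laser attacks.
; Roam, started from BeginPlay, re-runs on a short delay, reversing at traced obstacles and calling Chase when the player is near, without stopping itself.
; Chase loops similarly, turning toward the player via X-scale flipping and spawning a short-lived LaserBeam when a forward trace hits BP_Player.
; It falls back to Roam when out of range.
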(event Custom|Chase
  (bind _distance (CallFunction|GetPlayerDistance))
  (if (<= _distance 5e+02)
    (if (< (.x (Transformation|GetActorLocation)) (.x (Transformation|GetActorLocation (Game|GetPlayerCharacter 0))))
      (Variables|Default|SetMoveDirection "1.000000,0.000000,0.000000")
      (else
        (Variables|Default|SetMoveDirection "-1.000000,0.000000,0.000000")))
    (CallFunction|FlipCharacter)
    (bind _isdetected (CallFunction|DetectPlayer))
    (if _isdetected
      (CallFunction|Attack))
    (Variables|/Script/Engine.MovementComponent|SetVelocity (Variables|Character|GetCharacterMovement self) (* (Variables|Default|GetMoveDirection) 3e+02))
    (Utilities|FlowControl|Delay 0.2)
    (CallFunction|Chase)
    (else
      (CallFunction|Roam))))

(event Custom|Roam
  (bind _returnvalue (Transformation|GetActorLocation))
  ;[0.15 0.15 0.15 0.5] Roam
  (Variables|/Script/Engine.MovementComponent|SetVelocity (Variables|Character|GetCharacterMovement self) (* (Variables|Default|GetMoveDirection) 2e+02))
  (bind _returnvalue_2 (Collision|LineTraceByChannel _returnvalue (+ _returnvalue (* (Variables|Default|GetMoveDirection) 1e+02)) "TraceTypeQuery1" false 0 "ForDuration" true "(R=1.000000,G=0.000000,B=0.000000,A=1.000000)" "(R=0.000000,G=1.000000,B=0.000000,A=1.000000)" 2.0))
  (if _returnvalue_2
    (Variables|Default|SetMoveDirection (* (Variables|Default|GetMoveDirection) "-1.000000,1.000000,1.000000"))
    (CallFunction|FlipCharacter))
  (bind _distance (CallFunction|GetPlayerDistance))
  (if (<= _distance 5e+02)
    (CallFunction|Chase))
  (Utilities|FlowControl|Delay 0.2)
  (CallFunction|Roam))

(event Custom|Attack
  ;[0.15 0.15 0.15 0.5] Attack
  (bind _returnvalue (Game|SpawnActorfromClass "/Game/Blueprints/Characters/LaserBeam.LaserBeam_C" (Math|Transform|MakeTransform (+ (* (Variables|Default|GetMoveDirection) 2e+02) (Transformation|GetActorLocation)) "0, 0, 0" "1.500000,1.000000,1.000000") "Undefined" "MultiplyWithRoot" 0 0))
  (Actor|SetLifeSpan _returnvalue 1.0))

(event EventBeginPlay
  (switch Utilities|FlowControl|Switch|SwitchonEAIState (Variables|Default|GetAIState)
    (:NewEnumerator2
      (CallFunction|Roam))))

(event Collision|EventActorBeginOverlap
  (params (OtherActor :type Actor%20Object%20Reference)))

(event EventTick
  (params (DeltaSeconds :type Float%20%28single-precision%29)))

(fn ConstructionScript)

(fn FlipCharacter
  (bind _returnvalue (Class|Actor|GetActorRelativeScale3D))
  (Transformation|SetActorRelativeScale3D (Math|Vector|MakeVector (.x (Variables|Default|GetMoveDirection)) (.y _returnvalue) (.z _returnvalue))))

(fn DetectPlayer
  (bind _returnvalue (Transformation|GetActorLocation))
  (bind _outhit (Collision|LineTraceByChannel _returnvalue (+ _returnvalue (* (Variables|Default|GetMoveDirection) 2e+02)) "TraceTypeQuery1" false 0 "ForDuration" true "(R=1.000000,G=0.934981,B=0.000000,A=1.000000)" "(R=0.000000,G=0.202934,B=1.000000,A=1.000000)" 2.0))
  (Utilities|Casting|CastToBP_Player (.HitActor (Collision|BreakHitResult _outhit))
    (:then
      (return true))
    (:CastFailed
      (return false))))

(fn GetPlayerDistance
  (return (Math|Vector|Distance(Vector) (Transformation|GetActorLocation) (Transformation|GetActorLocation (Game|GetPlayerCharacter 0)))))