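; BP_Player is the side-view sprite player character, handling Enhanced Input movement, jump, attack and health.
; Tick raises gravity while falling and rebuilds buffed attack and cooldown from BuffComponent, applying additive before multiplicative modifiers.
; Attacks play an animation override gated by the base cooldown, not the buffed one; the hitbox's enemy overlap is a stub.
; Damage triggers timed invincibility, and debug inputs add a test buff or show GM_Rogue's UI.
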(event OnComponentBeginOverlap(Attack_0_box)
  (params (OverlappedComponent :type Primitive%20Component%20Object%20Reference) (OtherActor :type Actor%20Object%20Reference) (OtherComp :type Primitive%20Component%20Object%20Reference) (OtherBodyIndex :type Integer) (bFromSweep :type Boolean) (SweepResult :type Hit%20Result%20Structure%20%28by%20ref%29))
  (if (Actor|ActorHasTag OtherActor "Enemy")
    _))

(event Input|EnhancedActionEvents|EnhancedInputActionIA_Move
  (params (ActionValue :type Float%20%28double-precision%29) (ElapsedSeconds :type Float%20%28double-precision%29) (TriggeredSeconds :type Float%20%28double-precision%29) (InputAction :type Input%20Action%20Object%20Reference :default "/Game/Blueprints/Input/IA_Move.IA_Move"))
  (bind _sprite (Variables|Default|GetSprite))
  (Pawn|Input|AddMovementInput "1.000000,0.000000,0.000000" ActionValue false)
  (if (== ActionValue 1.0)
    (Transformation|SetRelativeRotation _sprite "0, 0, 0" false false)
    (else
      (Transformation|SetRelativeRotation _sprite "0.000000,180.000000,0.000000" false false))))

(event Input|EnhancedActionEvents|EnhancedInputActionIA_Jump
  (params (ActionValue :type Boolean) (ElapsedSeconds :type Float%20%28double-precision%29) (TriggeredSeconds :type Float%20%28double-precision%29) (InputAction :type Input%20Action%20Object%20Reference :default "/Game/Blueprints/Input/IA_Jump.IA_Jump"))
  (:Started
    (Character|Jump))
  (:Completed
    (Character|StopJumping)))

(event Input|EnhancedActionEvents|EnhancedInputActionIA_Attack
  (params (ActionValue :type Boolean) (ElapsedSeconds :type Float%20%28double-precision%29) (TriggeredSeconds :type Float%20%28double-precision%29) (InputAction :type Input%20Action%20Object%20Reference :default "/Game/Blueprints/Input/IA_Attack.IA_Attack"))
  (:Started
    (if (Variables|Default|GetCanAttack)
      (Utilities|FlowControl|Sequence
        (:then_0
          (|PlayAnimationOverridewithCallbacks (Variables|/Script/PaperZD.PaperZDAnimationComponent|GetAnimInstance (Variables|Default|GetAnimationComponent)) "/Game/Blueprints/Animation/AnimSequences/Attack_0.Attack_0" "AttackSlot" 1.0 0.0
            (:then
              (Variables|Default|SetCanAttack false)
              (Utilities|FlowControl|Delay (Variables|Default|GetBaseAttackCD))
              (Variables|Default|SetCanAttack true))))))))

(event Input|EnhancedActionEvents|EnhancedInputActionIA_GetBuff
  (params (ActionValue :type Boolean) (ElapsedSeconds :type Float%20%28double-precision%29) (TriggeredSeconds :type Float%20%28double-precision%29) (InputAction :type Input%20Action%20Object%20Reference :default "/Game/Blueprints/Input/IA_GetBuff.IA_GetBuff"))
  (:Started
    (Default|AddBuff (Variables|Default|GetBuff%20Component) (Variables|/Game/Data/Buffs/DA_BUFF.DA_BUFF_C|GetBuff_ATK_20%25_UP (Variables|Default|GetBuffTable)))
    (Utilities|FlowControl|DelayUntilNextTick)
    (Development|PrintString (Utilities|String|ToString(Float) (Variables|Default|GetBuffedAttack)))))

(event EventBeginPlay
  (CallFunction|InputSystemInit)
  (CallFunction|SetHealth (Variables|Default|GetBaseMaxHealth)))

(event Collision|EventActorBeginOverlap
  (params (OtherActor :type Actor%20Object%20Reference)))

(event EventTick
  (params (DeltaSeconds :type Float%20%28single-precision%29))
  (Utilities|FlowControl|Sequence
    (:then_0
      (|GravityUpdate_2))
    (:then_1
      (CallFunction|ApplyBuff))))

(event Game|Damage|EventAnyDamage
  (params (Damage :type Float%20%28single-precision%29) (DamageType :type Damage%20Type%20Object%20Reference) (InstigatedBy :type Controller%20Object%20Reference) (DamageCauser :type Actor%20Object%20Reference))
  (if (Variables|Default|GetCanBeHurt)
    (CallFunction|ChangeHealth (Math|Float|Truncate (* Damage -1.0)))
    (Variables|Default|SetCanBeHurt false)
    (Utilities|FlowControl|Delay (Variables|Default|GetBaseInvincibleCD))
    (Variables|Default|SetCanBeHurt true)))

(event EventOnJumped
  (Class|PaperZDAnimInstance|JumptoNode (Variables|/Script/PaperZD.PaperZDAnimationComponent|GetAnimInstance (Variables|Default|GetAnimationComponent)) "JumpState" "None"))

(event Input|KeyboardEvents|U
  (params (Key :type Key%20Structure :default "None"))
  (:Pressed
    (Development|PrintString "ShowUI")
    (bind _asgm_rogue (Utilities|Casting|CastToGM_Rogue (Game|GetGameMode)))
    (Development|PrintString "cast OK")
    (Default|ShowUI _asgm_rogue)))

(fn ConstructionScript)

(fn InputSystemInit
  (bind _asbp_player_controller (Utilities|Casting|CastToBP_PlayerController (Pawn|GetController)))
  (Utilities|IsValid (PlayerController|LocalPlayerSubsystems|GetEnhancedInputLocalPlayerSubsystem _asbp_player_controller)
    (:Is%20Valid
      (Input|AddMappingContext (PlayerController|LocalPlayerSubsystems|GetEnhancedInputLocalPlayerSubsystem _asbp_player_controller) "/Game/Blueprints/Input/IMC_Player.IMC_Player" 0 "(bIgnoreAllPressedKeysUntilRelease=True,bForceImmediately=False,bNotifyUserSettings=False)"))))

(fn SetHealth
  (params (health :type Integer))
  (Variables|Default|SetHealth (Math|Integer|Clamp(Integer) health 0 (Variables|Default|GetBaseMaxHealth))))

(fn ChangeHealth
  (params (changeAmount :type Integer))
  (CallFunction|SetHealth (+ (Variables|Default|GetHealth) changeAmount)))

(fn SetAttack0Box
  (params (boxStatus :type Boolean))
  (bind _attack_0_box (Variables|Default|GetAttack_0_box))
  (if boxStatus
    (Collision|SetCollisionEnabled _attack_0_box "QueryOnly")
    (else
      (Collision|SetCollisionEnabled _attack_0_box "NoCollision"))))

(fn CalDamage)

(fn ApplyBuff
  (bind _output_get (Variables|Default|SetBuffedAttack (Variables|Default|GetBaseAttack)))
  (bind _output_get_2 (Variables|Default|SetBuffedAttackCD (Variables|Default|GetBaseAttackCD)))
  (bind _buffs (Default|GetBuffs (Variables|Default|GetBuff%20Component)))
  (Utilities|FlowControl|Sequence
    (:then_0
      (for _array_element _buffs
        (Variables|Default|SetBuffedAttack (+ _output_get (.attackadd (.statmods (.buff_def _array_element)))))))
    (:then_1
      (for _array_element_2 _buffs
        (Variables|Default|SetBuffedAttack (* _output_get (.attackmul (.statmods (.buff_def _array_element_2)))))))
    (:then_2
      (for _array_element_3 _buffs
        (Variables|Default|SetBuffedAttackCD (* _output_get_2 (.attackspeedmul (.statmods (.buff_def _array_element_3)))))))))