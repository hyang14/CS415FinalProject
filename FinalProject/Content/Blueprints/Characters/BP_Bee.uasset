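; BP_Bee is a flipbook-animated flying enemy that pursues and attacks the player.
; Each Tick checks distance: in range it calls Attack after a Delay, otherwise Roam sets the fly flipbook and homes ProjectileMovement on the player's capsule.
; Attack launches the bee in X and Z using the player's normalized world position, not a relative direction.
; Capsule hits on BP_Player pass Damage to ChangeHealth, then call Roam.
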(event OnComponentHit(CapsuleComponent)
  (params (HitComponent :type Primitive%20Component%20Object%20Reference) (OtherActor :type Actor%20Object%20Reference) (OtherComp :type Primitive%20Component%20Object%20Reference) (NormalImpulse :type Vector :default "0, 0, 0") (Hit :type Hit%20Result%20Structure%20%28by%20ref%29))
  (bind _asbp_player (Utilities|Casting|CastToBP_Player OtherActor))
  (Default|ChangeHealth _asbp_player (Math|Float|Truncate (Variables|Default|Getdamage)))
  (CallFunction|Roam))

(event EventBeginPlay)

(event EventTick
  (params (DeltaSeconds :type Float%20%28single-precision%29))
  (if (<= (Math|Vector|Distance(Vector) (Transformation|GetWorldLocation (Variables|Collision|GetCapsuleComponent)) (Transformation|GetWorldLocation (Variables|/Script/Engine.Actor|GetRootComponent (Game|GetPlayerCharacter 0)))) 5e+02)
    (Utilities|FlowControl|Delay 2.0)
    (CallFunction|Attack)
    (else
      (CallFunction|Roam))))

(fn ConstructionScript)

(fn Attack
  (Sprite|SetFlipbook (Variables|Default|GetSprite) "/Game/Mob/Small_Bee/Attack/FB_Bee_Attack.FB_Bee_Attack")
  (Character|LaunchCharacter (* (Math|Vector|Normalize (Transformation|GetWorldLocation (Variables|/Script/Engine.Actor|GetRootComponent (Game|GetPlayerCharacter 0)))) "500.000000,0.000000,500.000000") false false))

(fn Roam
  (Sprite|SetFlipbook (Variables|Default|GetSprite) "/Game/Mob/Small_Bee/Fly/FB_Bee_Fly.FB_Bee_Fly")
  (bind _asbp_player (Utilities|Casting|CastToBP_Player (Game|GetPlayerCharacter 0)))
  (Variables|/Script/Engine.ProjectileMovementComponent|SetHomingTargetComponent (Variables|Default|GetProjectileMovement) (Variables|/Script/Engine.Character|GetCapsuleComponent _asbp_player)))